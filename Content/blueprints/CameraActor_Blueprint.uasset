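; Camera actor that creeps along its relative Z axis and destroys characters that touch its box trigger.
; Tick calls MoveComponentTo to offset the camera component by a fixed step whenever the frame delta differs from the stored Time value.
; The box overlap spawns an explosion at any actor tagged "Chara", then destroys that actor.
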(event OnComponentBeginOverlap(Box)
  (params (OtherActor :type Actor%20Object%20Reference) (OtherComp :type Primitive%20Component%20Object%20Reference) (OtherBodyIndex :type Integer) (bFromSweep :type Boolean) (SweepResult :type Hit%20Result%20Structure%20%28by%20ref%29))
  (if (Actor|ActorHasTag OtherActor "Chara")
    (Effects|SpawnEmitteratLocation "/Game/StarterContent/Particles/P_Explosion.P_Explosion" (Transformation|GetActorLocation OtherActor))
    (Actor|SetLifeSpan OtherActor 0.0)
    (Actor|DestroyActor OtherActor)))

(event EventActorBeginOverlap
  (params (OtherActor :type Actor%20Object%20Reference)))

(event EventTick
  (params (DeltaSeconds :type Float%20%28single-precision%29)))

(event EventTick
  (params (DeltaSeconds :type Float%20%28single-precision%29))
  (if (not (== DeltaSeconds (Variables|Default|Gettime)))
    (Variables|Default|Settime (Utilities|Time|GetWorldDeltaSeconds))
    (Components|MoveComponentTo (Variables|CameraActor|GetCameraComponent) (+ (Variables|/Script/Engine.SceneComponent|GetRelativeLocation (Variables|CameraActor|GetCameraComponent)) "0.000000,0.000000,5.000000") (Variables|/Script/Engine.SceneComponent|GetRelativeRotation (Variables|CameraActor|GetCameraComponent)) false false 0.2)))

(fn ConstructionScript)